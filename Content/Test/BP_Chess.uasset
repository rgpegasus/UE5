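; Test actor for a "chess" (apparently a chest) that opens when the player stands inside its box trigger and faces it.
; While the player overlaps the box, Tick compares the player's forward vector with the chess-to-player direction using a dot product threshold.
; A timeline pitches the Pivot component to open and reverses to close when the player looks away or leaves, guarded by an IsClose flag.
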(event `self.Box.OnComponentBeginOverlap`
  (params (OverlappedComponent :type "PrimitiveComponent Object Reference") (OtherActor :type "Actor Object Reference") (OtherComp :type "PrimitiveComponent Object Reference") (OtherBodyIndex :type Integer) (bFromSweep :type Boolean) (SweepResult :type "HitResult Structure (by ref)"))
  ; Player enter the Hit Box
  (if (== OtherActor (`GameplayStatics.GetPlayerCharacter` 0))
    (set `self.PlayerIn` true)))

(event `self.Box.OnComponentEndOverlap`
  (params (OverlappedComponent :type "PrimitiveComponent Object Reference") (OtherActor :type "Actor Object Reference") (OtherComp :type "PrimitiveComponent Object Reference") (OtherBodyIndex :type Integer))
  ; Player leave the Hit Box
  (if (== OtherActor (`GameplayStatics.GetPlayerCharacter` 0))
    (set `self.PlayerIn` false)
    (`self.ChessAnimation` false)))

(event `self.ReceiveTick`
  (params (DeltaSeconds :type "Float (single-precision)"))
  ; Test if the player is looking at the chess
  (if (`self.PlayerIn`)
    (bind _chess_playervector (`self.GetChess-PlayerVector`))
    (`self.ChessAnimation` (< (`KismetMathLibrary.Dot_VectorVector` _chess_playervector (`KismetMathLibrary.Normal` (`KismetMathLibrary.GetForwardVector` (`self.K2_GetActorRotation` (`GameplayStatics.GetPlayerCharacter` 0))))) -0.5))))

(event `ChessAnimation`
  (params (PlayerIsFacing :type Boolean))
  ; Open and close the chess
  (if PlayerIsFacing
    (if (`self.IsClose`)
      (set `self.IsClose` false)
      (bind (_direction _rotationy) (`Timeline|Timeline` :!label _label)
        (:`Update`
          (`SceneComponent.K2_SetRelativeRotation` (`self.Pivot`) (`KismetMathLibrary.MakeRotator` 0.0 _rotationy) false false))))
    (elif (not (`self.IsClose`))
      (set `self.IsClose` true)
      (goto _label :!via `Reverse`))))

(fn `GetChess-PlayerVector`
  (returns (`Chess-PlayerVector` :type "Vector Structure"))
  (return (`KismetMathLibrary.GetDirectionUnitVector` (`self.K2_GetActorLocation`) (`self.K2_GetActorLocation` (`GameplayStatics.GetPlayerCharacter` 0)))))

(fn `UserConstructionScript`)